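; BP_Navlink is a smart nav link that launches enemy characters into a timed jump when they reach it.
; On SmartLinkReached, it casts the agent to Enemy_Character and passes its location, the link destination and a jump time to GetJumpVelocity.
; That function derives velocity from start-minus-end offsets over time, with hardcoded gravity compensation on Z.
; LaunchCharacter applies the result, overriding XY and Z velocity.
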(event `self.ReceiveSmartLinkReached`
  (params (Agent :type "Actor Object Reference") (Destination :type "Vector Structure (by ref)"))
  (bind _asenemy_character (cast `/Game/EnemyAI/Enemy_Character` Agent))
  (bind _jumpvelocity (`self.GetJumpVelocity` (`self.K2_GetActorLocation` _asenemy_character) Destination (`self.JumpTIme`)))
  (`Character.LaunchCharacter` _asenemy_character _jumpvelocity true true))

(fn `GetJumpVelocity`
  (params (StartingLocation :type "Vector Structure") (EndLocation :type "Vector Structure") (JumpTime :type "Float (double-precision)"))
  (returns (JumpVelocity :type "Vector Structure"))
  (locals (SetDuration :type "Float (double-precision)"))
  (bind _setduration (`local.SetDuration`))
  (bind _setduration_2 (`local.SetDuration`))
  (set `local.SetDuration` JumpTime)
  (return (`KismetMathLibrary.MakeVector` (/ (- (.x StartingLocation) (.x EndLocation)) _setduration_2) (/ (- (.y StartingLocation) (.y EndLocation)) _setduration_2) (/ (- (.z StartingLocation) (+ (.z EndLocation) (* (`KismetMathLibrary.Square` _setduration) -0.5 982.0))) _setduration))))

(fn `UserConstructionScript`)